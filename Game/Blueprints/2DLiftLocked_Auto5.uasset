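; 2D lift that moves its sprite between its origin and an editable EndLocation on a timeline, with play rate set from TravelTimeSec.
; When the timeline finishes, it waits StopDelay and runs again in the opposite direction.
; A character overlapping the safety collider calls Play or Reverse on an active timeline, depending on whether it is playing.
; The construction script can place the sprite at EndLocation for preview via TestEndLocation.
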(event OnComponentBeginOverlap(SafteyCollider)
  (params (OverlappedComponent :type Primitive%20Component%20Object%20Reference) (OtherActor :type Actor%20Object%20Reference) (OtherComp :type Primitive%20Component%20Object%20Reference) (OtherBodyIndex :type Integer) (bFromSweep :type Boolean) (SweepResult :type Hit%20Result%20Structure%20%28by%20ref%29))
  (bind _lift_timeline (Variables|Default|GetLift%20Timeline))
  ;[1 1 1] Defines how the lift moves
  (Utilities|Casting|CastToMyCharacter OtherActor)
  (if (Components|Activation|IsActive _lift_timeline)
    (if (Audio|Components|Audio|IsPlaying _lift_timeline)
      (bind (_direction _lerp_alpha) (Timeline|Lift%20Timeline Play)
        (:Update
          (Transformation|SetRelativeLocation (Variables|Default|GetLiftSprite) (Math|Vector|Lerp(Vector) "0, 0, 0" (Variables|LiftControls|GetEndLocation) _lerp_alpha) false false))
        (:Finished
          (Utilities|FlowControl|Delay (Variables|LiftControls|GetStop%20Delay))
          (switch Utilities|FlowControl|Switch|SwitchonETimelineDirection _direction
            (:Forward
              (CallFunction|LiftBack))
            (:Backward
              (CallFunction|LiftForward)))))
      (else
        (Timeline|Lift%20Timeline Reverse)))))

(event Custom|LiftForward
  ;[1 1 1] Defines how the lift moves
  (bind (_direction _lerp_alpha) (Timeline|Lift%20Timeline PlayFromStart)
    (:Update
      (Transformation|SetRelativeLocation (Variables|Default|GetLiftSprite) (Math|Vector|Lerp(Vector) "0, 0, 0" (Variables|LiftControls|GetEndLocation) _lerp_alpha) false false))
    (:Finished
      (Utilities|FlowControl|Delay (Variables|LiftControls|GetStop%20Delay))
      (switch Utilities|FlowControl|Switch|SwitchonETimelineDirection _direction
        (:Forward
          (CallFunction|LiftBack))
        (:Backward
          (CallFunction|LiftForward))))))

(event Custom|LiftBack
  ;[1 1 1] Defines how the lift moves
  (bind (_direction _lerp_alpha) (Timeline|Lift%20Timeline ReverseFromEnd)
    (:Update
      (Transformation|SetRelativeLocation (Variables|Default|GetLiftSprite) (Math|Vector|Lerp(Vector) "0, 0, 0" (Variables|LiftControls|GetEndLocation) _lerp_alpha) false false))
    (:Finished
      (Utilities|FlowControl|Delay (Variables|LiftControls|GetStop%20Delay))
      (switch Utilities|FlowControl|Switch|SwitchonETimelineDirection _direction
        (:Forward
          (CallFunction|LiftBack))
        (:Backward
          (CallFunction|LiftForward))))))

(event Collision|EventActorBeginOverlap
  (params (OtherActor :type Actor%20Object%20Reference)))

(event EventTick
  (params (DeltaSeconds :type Float%20%28single-precision%29)))

(event EventBeginPlay
  ;[1 1 1] defines travel times and a changable end location
  (Components|Timeline|SetPlayRate (Variables|Default|GetLift%20Timeline) (/ 1.0 (Variables|LiftControls|GetTravelTimeSec)))
  (Variables|LiftControls|SetTestEndLocation true))

(fn ConstructionScript
  ;[1 1 1] allows a testable end location
  (Transformation|SetRelativeLocation (Variables|Default|GetLiftSprite) (Math|Vector|SelectVector (Variables|LiftControls|GetEndLocation) "0, 0, 0" (Variables|LiftControls|GetTestEndLocation)) false false))