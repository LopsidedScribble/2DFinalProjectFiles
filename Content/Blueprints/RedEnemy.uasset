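; RedEnemy is a 2D flipbook enemy that patrols between two points and knocks the player back on contact.
; The construction script feeds PointA and PointB as relative control points into the BasicEnemyMove interp movement component.
; Each movement reversal toggles the flipbook's rotation through a FlipFlop to turn the sprite around.
; Capsule overlap launches MyCharacter upward and along X using the sweep normal, without applying damage despite the graph comment.
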(event OnInterptoReverse(BasicEnemyMove)
  (params (ImpactResult :type Hit%20Result%20Structure%20%28by%20ref%29) (Time :type Float%20%28single-precision%29))
  (bind _run_flipbook (Variables|Default|GetRun_flipbook))
  ;[1 1 1] Sets the flipbook rotation at end of movement
  (Utilities|FlowControl|FlipFlop
    (:A
      (Transformation|SetWorldRotation _run_flipbook "0,180.000000, 0" false false))
    (:B
      (Transformation|SetWorldRotation _run_flipbook "0, 0, 0" false false))))

(event OnComponentBeginOverlap(Capsule)
  (params (OverlappedComponent :type Primitive%20Component%20Object%20Reference) (OtherActor :type Actor%20Object%20Reference) (OtherComp :type Primitive%20Component%20Object%20Reference) (OtherBodyIndex :type Integer) (bFromSweep :type Boolean) (SweepResult :type Hit%20Result%20Structure%20%28by%20ref%29))
  ;[1 1 1] Damages and launches character
  (bind _asmy_character (Utilities|Casting|CastToMyCharacter OtherActor))
  (Character|LaunchCharacter _asmy_character (Math|Vector|MakeVector (* (.x (.Normal (Collision|BreakHitResult SweepResult))) -1e+03) 0.0 2e+02) true true))

(event EventBeginPlay)

(event Collision|EventActorBeginOverlap
  (params (OtherActor :type Actor%20Object%20Reference)))

(event EventTick
  (params (DeltaSeconds :type Float%20%28single-precision%29)))

(fn ConstructionScript
  (Variables|/Script/Engine.InterpToMovementComponent|SetControlPoints (Variables|Default|GetBasicEnemyMove) (Utilities|Array|MakeArray (Utilities|Struct|MakeInterpControlPoint (Variables|Default|GetPoint%20A) true) (Utilities|Struct|MakeInterpControlPoint (Variables|Default|GetPoint%20B) true))))